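; BP_OrbitPawn is an orbit camera pawn for inspecting info actors in dioramas.
; Move axes rotate OrbitArm and re-aim the camera at it.
; While possessed, it traces under the cursor each Tick for hover and on right-click release for selection, delegating both to the parent diorama.
; The selection result toggles title and subtitle text; background hits clear hover or selection across all GameInstance dioramas.
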(event `Key|E`
  (params (Key :type "Key Structure" :default "AnyKey"))
  (:`Released`
    ;[1 1 1] Hover code
    ;;[0 0.3864 0.8796] If player hovers over something not an infoActor (i.e., the background) , tell all dioramas to unhover all infoActors
    (bind _asbp_game_instance (cast `/Game/Neurorama/Core/BP_GameInstance` (`GameplayStatics.GetGameInstance`) :!label _label))
    (for _array_element (`/Game/Neurorama/Core/BP_GameInstance.dioramasCollected` _asbp_game_instance)
      (bind _asbp_diorama_master (cast `/Game/Neurorama/InfoActors/bp_Diorama_Master` _array_element))
      (`/Game/Neurorama/InfoActors/bp_Diorama_Master.unhoverAllInfoActors` _asbp_diorama_master))))

(event `InputAxis|MoveForward`
  (params (AxisValue :type "Float (single-precision)"))
  ;[1 1 1] Rotation Control
  (`SceneComponent.K2_AddLocalRotation` (`self.OrbitArm`) (`KismetMathLibrary.MakeRotator` 0.0 AxisValue) false false)
  (`SceneComponent.K2_SetWorldRotation` (`self.Camera`) (`KismetMathLibrary.MakeRotator` (.roll (`SceneComponent.K2_GetComponentRotation` (`self.OrbitArm`))) (.pitch (`KismetMathLibrary.FindLookAtRotation` (`SceneComponent.K2_GetComponentLocation` (`self.Camera`)) (`SceneComponent.K2_GetComponentLocation` (`self.OrbitArm`)))) (.yaw (`KismetMathLibrary.FindLookAtRotation` (`SceneComponent.K2_GetComponentLocation` (`self.Camera`)) (`SceneComponent.K2_GetComponentLocation` (`self.OrbitArm`))))) false false :!label _label_2))

(event `self.ReceiveTick`
  (params (DeltaSeconds :type "Float (single-precision)"))
  (bind (_bblockinghit _binitialoverlap _time _location _impactpoint _normal _impactnormal _physmat _hitactor) (`GameplayStatics.BreakHitResult` (`PlayerController.GetHitResultUnderCursorByChannel` (`GameplayStatics.GetPlayerController` 0) "TraceTypeQuery1" true)))
  ;[1 1 1] Hover code
  ;;[0.1746 0.006512 0.006512] Mouse hover over infoActor code
  (`self.isPawnControlled?`
    (:`IsControlled`
      (bind _asbp_ia_master (cast `/Game/Neurorama/InfoActors/BP_ia_Master` _hitactor) ; Was the object selected an infoActor?
        (:`then`
          ;;[0.07819 0.1845 0.2831] Tell Diorama that owns hit object to select it if it is an infoActor
          (bind _asbp_diorama_master (cast `/Game/Neurorama/InfoActors/bp_Diorama_Master` (`self.GetParentActor` _hitactor))) ; Cast to diorama which owns the infoActor, because dioramas contain a lot of the UX/UI code for infoActor display methods, just to keep things organized
          (`/Game/Neurorama/InfoActors/bp_Diorama_Master.hoverOverInfoActor` _asbp_diorama_master _asbp_ia_master))
        (:`CastFailed`
          (goto _label))))))

(event `InputAxis|MoveRight`
  (params (AxisValue :type "Float (single-precision)"))
  ;[1 1 1] Rotation Control
  (`SceneComponent.K2_AddWorldRotation` (`self.OrbitArm`) (`KismetMathLibrary.MakeRotator` 0.0 0.0 AxisValue) false false)
  (goto _label_2))

(event `Key|RightMouseButton`
  (params (Key :type "Key Structure" :default "AnyKey"))
  (bind (_bblockinghit _binitialoverlap _time _location _impactpoint _normal _impactnormal _physmat _hitactor) (`GameplayStatics.BreakHitResult` (`PlayerController.GetHitResultUnderCursorByChannel` (`GameplayStatics.GetPlayerController` 0) "TraceTypeQuery1" true)))
  ;[1 1 1] Selection code
  ;;[0.162 0.02029 0.02029] Mouse selecting infoActor code
  (:`Released`
    (`self.isPawnControlled?`
      (:`IsControlled`
        (cast `/Game/Neurorama/InfoActors/BP_ia_Master` _hitactor ; Was the object selected an infoActor?
          (:`then`
            ;;[0.0648 0.1651 0.2623] Tell Diorama that owns hit object to select it if it is an infoActor
            (bind _asbp_diorama_master (cast `/Game/Neurorama/InfoActors/bp_Diorama_Master` (`self.GetParentActor` _hitactor)))
            (bind _isdeselectingall (`/Game/Neurorama/InfoActors/bp_Diorama_Master.selectInfoActor` _asbp_diorama_master _location _hitactor))
            (if (== _isdeselectingall true)
              ;;[0.7379 0.1912 0.3712] Update HUD Information
              (`SceneComponent.SetVisibility` (`self.textTitle`) false false :!label _label_3)
              (`SceneComponent.SetVisibility` (`self.textSubtitle`) false false)
              (else
                (bind _asbp_ia_master (cast `/Game/Neurorama/InfoActors/BP_ia_Master` _hitactor))
                (`TextRenderComponent.K2_SetText` (`self.textTitle`) (`/Game/Neurorama/InfoActors/BP_ia_Master.Name` _asbp_ia_master))
                (`SceneComponent.SetVisibility` (`self.textTitle`) true false)
                (`TextRenderComponent.K2_SetText` (`self.textSubtitle`) (`/Game/Neurorama/InfoActors/BP_ia_Master.Description` _asbp_ia_master))
                (`SceneComponent.SetVisibility` (`self.textSubtitle`) true false))))
          (:`CastFailed`
            ;;[0 0.3864 0.8796] If player clicks on something not an infoActor (i.e., the background) , tell all dioramas to deselct all infoActors
            (bind _asbp_game_instance (cast `/Game/Neurorama/Core/BP_GameInstance` (`GameplayStatics.GetGameInstance`)))
            (for _array_element (`/Game/Neurorama/Core/BP_GameInstance.dioramasCollected` _asbp_game_instance)
              (bind _asbp_diorama_master_2 (cast `/Game/Neurorama/InfoActors/bp_Diorama_Master` _array_element))
              (`/Game/Neurorama/InfoActors/bp_Diorama_Master.deselectAllInfoActors` _asbp_diorama_master_2)
              (goto _label_3))))))))

(fn `UserConstructionScript`)