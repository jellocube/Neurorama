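; Desktop walk pawn for exploring dioramas, with axis-driven look and movement and a V key that spawns and possesses BP_Flypawn_Desktop.
; Camera line traces find info actors each tick for gaze hover and on right-click release for selection, delegating to the owning diorama.
; Selection toggles title and description text; misses clear hover or selection across all GameInstance dioramas.
; Click and touch set a Thrusting flag, but its movement code is unconnected.
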(event `InputAction|Action`
  (params (Key :type "Key Structure" :default "AnyKey"))
  (bind _movementenabled (`self.movementEnabled`))
  ;[1 1 1] Mouse & Touchpad Movement Control
  (:`Pressed`
    (if _movementenabled :!label _label
      (set `self.Thrusting` true)))
  (:`Released`
    (if _movementenabled :!label _label_2
      (set `self.Thrusting` false))))

(event `InputTouch`
  (params (Location :type "Vector Structure") (FingerIndex :type "ETouchIndex Enum"))
  ;[1 1 1] Mouse & Touchpad Movement Control
  (:`Pressed`
    (goto _label))
  (:`Released`
    (goto _label_2)))

(event `InputAxis|LookUp`
  (params (AxisValue :type "Float (single-precision)"))
  ;[1 1 1] Look Control
  (`self.AddControllerPitchInput` AxisValue))

(event `InputAxis|MoveForward`
  (params (AxisValue :type "Float (single-precision)"))
  ;[1 1 1] Movement input basic
  (`self.AddMovementInput` (`KismetMathLibrary.GetForwardVector` (`KismetMathLibrary.MakeRotator` 0.0 (.pitch (`self.GetControlRotation`)) (.yaw (`self.GetControlRotation`)))) (* AxisValue 0.5)))

(event `InputAxis|Turn`
  (params (AxisValue :type "Float (single-precision)"))
  ;[1 1 1] Look Control
  (`self.AddControllerYawInput` AxisValue))

(event `InputAxis|MoveRight`
  (params (AxisValue :type "Float (single-precision)"))
  ;[1 1 1] Movement input basic
  (`self.AddMovementInput` (`KismetMathLibrary.GetRightVector` (`KismetMathLibrary.MakeRotator` 0.0 (.pitch (`self.GetControlRotation`)) (.yaw (`self.GetControlRotation`)))) AxisValue))

(event `Key|V`
  (params (Key :type "Key Structure" :default "AnyKey"))
  ;[0.117 0.2346 0.1046] VR mode toggle
  (:`Pressed`
    (bind _returnvalue (`|SpawnActorFromClass` "/Game/Neurorama/UX/Pawns/BrokenPawns/BP_Flypawn_Desktop.BP_Flypawn_Desktop_C" (`self.GetTransform` (`GameplayStatics.GetPlayerController` 0)) "Undefined" "OverrideRootScale"))
    (`self.K2_TeleportTo` _returnvalue (`self.K2_GetActorLocation`) (`self.K2_GetActorRotation`))
    (bind _asplayer_controller (cast `PlayerController` (`GameplayStatics.GetPlayerController` 0)))
    (`Controller.Possess` _asplayer_controller _returnvalue)))

(event `Key|RightMouseButton`
  (params (Key :type "Key Structure" :default "AnyKey"))
  (bind _camera (`self.Camera`))
  (bind _returnvalue (`SceneComponent.K2_GetComponentLocation` _camera))
  ;[1 1 1] Selection code
  ;;[0.1746 0.006512 0.006512] Click-to-select infoActor code
  (:`Released`
    (`self.isPawnControlled?`)
    (bind _outhit (`KismetSystemLibrary.LineTraceSingle` _returnvalue (+ _returnvalue (* (`SceneComponent.GetForwardVector` _camera) 1000000.0)) "TraceTypeQuery2" false (`self.GetOverlappingActors` self null)))
    (bind (_bblockinghit _binitialoverlap _time _location _impactpoint _normal _impactnormal _physmat _hitactor) (`GameplayStatics.BreakHitResult` _outhit))
    (bind _asbp_ia_master (cast `/Game/Neurorama/InfoActors/BP_ia_Master` _hitactor)
      (:`then`
        ;;[0.0648 0.1651 0.2623] Tell Diorama that owns hit object to select it if it is an infoActor
        (bind _asbp_diorama_master (cast `/Game/Neurorama/InfoActors/bp_Diorama_Master` (`self.GetParentActor` _asbp_ia_master)))
        (bind _isdeselectingall (`/Game/Neurorama/InfoActors/bp_Diorama_Master.selectInfoActor` _asbp_diorama_master _location _asbp_ia_master))
        (if (== _isdeselectingall true)
          ;;[0.7379 0.1912 0.3712] Update HUD Information
          (`SceneComponent.SetVisibility` (`self.textTitle`) false false :!label _label_3)
          (`SceneComponent.SetVisibility` (`self.textSubtitle`) false false)
          (else
            (bind _asbp_ia_master_2 (cast `/Game/Neurorama/InfoActors/BP_ia_Master` _asbp_ia_master))
            (`TextRenderComponent.K2_SetText` (`self.textTitle`) (`/Game/Neurorama/InfoActors/BP_ia_Master.Name` _asbp_ia_master_2))
            (`SceneComponent.SetVisibility` (`self.textTitle`) true false)
            (`TextRenderComponent.K2_SetText` (`self.textSubtitle`) (`/Game/Neurorama/InfoActors/BP_ia_Master.Description` _asbp_ia_master_2))
            (`SceneComponent.SetVisibility` (`self.textSubtitle`) true false))))
      (:`CastFailed`
        ;;[0 0.3864 0.8796] If player clicks on something not an infoActor (i.e., the background) , tell all dioramas to deselct all infoActors
        (bind _asbp_game_instance (cast `/Game/Neurorama/Core/BP_GameInstance` (`GameplayStatics.GetGameInstance`)))
        (for _array_element (`/Game/Neurorama/Core/BP_GameInstance.dioramasCollected` _asbp_game_instance)
          (bind _asbp_diorama_master_2 (cast `/Game/Neurorama/InfoActors/bp_Diorama_Master` _array_element))
          (`/Game/Neurorama/InfoActors/bp_Diorama_Master.deselectAllInfoActors` _asbp_diorama_master_2)
          (goto _label_3))))))

(event `self.ReceiveTick`
  (params (DeltaSeconds :type "Float (single-precision)"))
  (bind _camera (`self.Camera`))
  (bind _returnvalue (`SceneComponent.K2_GetComponentLocation` _camera))
  ;[1 1 1] Gaze-based hover-highlighting code
  ;;[0.1441 0.006512 0.006049] Line trace from player viewpoint and see if it intersects with a BPia
  (`self.isPawnControlled?`)
  (bind _outhit (`KismetSystemLibrary.LineTraceSingle` _returnvalue (+ _returnvalue (* (`SceneComponent.GetForwardVector` _camera) 1000000.0)) "TraceTypeQuery2" false (`self.GetOverlappingActors` self null)))
  (bind (_bblockinghit _binitialoverlap _time _location _impactpoint _normal _impactnormal _physmat _hitactor) (`GameplayStatics.BreakHitResult` _outhit))
  (bind _asbp_ia_master (cast `/Game/Neurorama/InfoActors/BP_ia_Master` _hitactor)
    (:`then`
      ;;[0.07819 0.1845 0.2831] Tell Diorama that owns hit object that it is hovered over it if it is an infoActor
      (bind _asbp_diorama_master (cast `/Game/Neurorama/InfoActors/bp_Diorama_Master` (`self.GetParentActor` _hitactor))) ; Cast to diorama which owns the infoActor, because dioramas contain a lot of the UX/UI code for infoActor display methods, just to keep things organized
      (`/Game/Neurorama/InfoActors/bp_Diorama_Master.hoverOverInfoActor` _asbp_diorama_master _asbp_ia_master))
    (:`CastFailed`
      ;;[0 0.3864 0.8796] If player hovers over something not an infoActor (i.e., the background) , tell all dioramas to unhover all infoActors
      (bind _asbp_game_instance (cast `/Game/Neurorama/Core/BP_GameInstance` (`GameplayStatics.GetGameInstance`)))
      (for _array_element (`/Game/Neurorama/Core/BP_GameInstance.dioramasCollected` _asbp_game_instance)
        (bind _asbp_diorama_master_2 (cast `/Game/Neurorama/InfoActors/bp_Diorama_Master` _array_element))
        (`/Game/Neurorama/InfoActors/bp_Diorama_Master.unhoverAllInfoActors` _asbp_diorama_master_2)))))

(fn `UserConstructionScript`)