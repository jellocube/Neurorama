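; BP_Menupawn_VR is a VR menu pawn that lets the player click 3D widgets.
; On PrimaryButton press, its WidgetInteraction component sends an immediate left-mouse press and release if it is over an interactable widget.
; An isPawnControlled? graph checks whether the pawn is possessed by player controller 0, though the event graph does not call it.
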(event `InputAction|PrimaryButton`
  (params (Key :type "Key Structure"))
  ;[1 1 1] Allow clicking 3D widgets via Widget Interaction
  (:`Pressed`
    (if (`WidgetInteractionComponent.IsOverInteractableWidget` (`self.WidgetInteraction`))
      (`WidgetInteractionComponent.PressPointerKey` (`self.WidgetInteraction`) "LeftMouseButton")
      (`WidgetInteractionComponent.ReleasePointerKey` (`self.WidgetInteraction`) "LeftMouseButton"))))

(fn `UserConstructionScript`)