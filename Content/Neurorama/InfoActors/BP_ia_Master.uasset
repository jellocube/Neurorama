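; Master InfoActor for Neurorama: a selectable, data-driven mesh with name and description that registers itself with BP_GameInstance on BeginPlay.
; The construction script fills colors and text from DT_iaSheet by class name, trimming four trailing characters for asymmetric hemisphere meshes and printing missing rows.
; Engage, gaze and reveal/hide events play or reverse timelines driving material highlight and opacity parameters.
; Hiding also disables collision so pointer selection ignores hidden actors.
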(event `self.ReceiveBeginPlay`
  ;[0 0.6654 1] At begin play, add all infoActors to an array in the Game Instance
  (bind _asbp_game_instance (cast `/Game/Neurorama/Core/BP_GameInstance` (`GameplayStatics.GetGameInstance`)))
  (`KismetArrayLibrary.Array_Add` (`/Game/Neurorama/Core/BP_GameInstance.infoActorsCollected` _asbp_game_instance) self)
  ;[1 1 1] By disabling collision, mouse and pointer selection won't affect hidden actors
  (`PrimitiveComponent.SetCollisionEnabled` (`self.InfoActMesh`) "QueryAndPhysics" :!label _label)
  (bind (_direction _visibilityrevealetccurve) (`Timeline|changeOpacity` :!label _label_2)
    (:`Update`
      (`MeshComponent.SetScalarParameterValueOnMaterials` (`self.InfoActMesh`) "Opacity" (`KismetMathLibrary.Lerp` _visibilityrevealetccurve)))))

(event `/Game/Neurorama/InfoActors/BPI_infoInterfaces.EngageInfoActor`
  ;[1 1 1] Code to highlight infoActors when engaged (clicked)
  (bind (_direction _gotcurvescurve) (`Timeline|selectionHighlight` :!label _label_3)
    (:`Update`
      (`MeshComponent.SetScalarParameterValueOnMaterials` (`self.InfoActMesh`) "selectValue" (`KismetMathLibrary.Lerp` _gotcurvescurve (`self.HighlightIntensity`))))))

(event `/Game/Neurorama/InfoActors/BPI_infoInterfaces.DisengageInfoActor`
  ;[1 1 1] Code to highlight infoActors when engaged (clicked)
  (goto _label_3 :!via `Reverse`))

(event `/Game/Neurorama/InfoActors/BPI_infoInterfaces.gazeHover`
  ;[1 1 1] Code to hoverhighlight objects when gazed upon
  (bind (_direction _linearrise) (`Timeline|hoverHighlight` :!label _label_4)
    (:`Update`
      (`MeshComponent.SetScalarParameterValueOnMaterials` (`self.InfoActMesh`) "hoverValue" (`KismetMathLibrary.Lerp` _linearrise (`self.HoverIntensity`))))))

(event `/Game/Neurorama/InfoActors/BPI_infoInterfaces.gazeIgnore`
  ;[1 1 1] Code to hoverhighlight objects when gazed upon
  (goto _label_4 :!via `Reverse`))

(event `HideActor`
  ;[1 1 1] By disabling collision, mouse and pointer selection won't affect hidden actors
  (`PrimitiveComponent.SetCollisionEnabled` (`self.InfoActMesh`) "NoCollision")
  (goto _label_2 :!via `Reverse`))

(event `Reveal Actor`
  (goto _label))

(fn `UserConstructionScript`
  (locals (NewLocalVar_0 :type "Material Object Reference"))
  (bind _returnvalue (`KismetSystemLibrary.GetClassDisplayName` (`GameplayStatics.GetObjectClass` self)))
  (bind _returnvalue_2 (`KismetStringLibrary.Concat_StrStr` (`KismetStringLibrary.LeftChop` (`KismetSystemLibrary.GetClassDisplayName` (`GameplayStatics.GetObjectClass` self)) 4)))
  ;[1 1 1] Create dynamic material instance(s)
  (`KismetMaterialLibrary.CreateDynamicMaterialInstance` (`PrimitiveComponent.GetMaterial` (`self.InfoActMesh`) 0))
  ;[1 1 1] Look up infoActor color in CSV datatable
  ;;[1 1 1] This splits asymmetric geometry betwen the hemispheres
  (if (`self.isAsymmetrical`)
    (bind _returnvalue_3 (`|GetDataTableRow` "/Game/Neurorama/InfoActors/DT_iaSheet.DT_iaSheet" (`KismetStringLibrary.Conv_StringToName` _returnvalue_2))
      (:`then`
        (bind (_color _secondary_color _display_name _description) (break `/Game/Neurorama/InfoActors/Sia_Array` _returnvalue_3))
        ;[1 1 1] InfoActors with asymmetrical mesh pairs
        ;;[1 1 1] Set colors
        (`MeshComponent.SetVectorParameterValueOnMaterials` (`self.InfoActMesh`) "PrimaryColor" (`KismetMathLibrary.Conv_LinearColorToVector` (`KismetStringLibrary.Conv_StringToColor` _color))) ; Functionality: any vector with name "PrimaryColor" in a material blueprint will be colored..
        (`MeshComponent.SetVectorParameterValueOnMaterials` (`self.InfoActMesh`) "SecondaryColor" (`KismetMathLibrary.Conv_LinearColorToVector` (`KismetStringLibrary.Conv_StringToColor` _secondary_color)))
        ;;[1 1 1] Set InfoActor name and description
        (set `self.Name` (`KismetTextLibrary.Conv_StringToText` _display_name))
        (set `self.Description` (`KismetTextLibrary.Conv_StringToText` _description)))
      (:`RowNotFound`
        (`KismetSystemLibrary.PrintString` _returnvalue_2 true true (struct :`R` 0.969136 :`B` 1.0 :`A` 1.0) 15.0) ; print out missing infoActor references
      ))
    (else
      (bind _returnvalue_4 (`|GetDataTableRow` "/Game/Neurorama/InfoActors/DT_iaSheet.DT_iaSheet" (`KismetStringLibrary.Conv_StringToName` _returnvalue)) ; This table contains all of the InfoActor  information.
        (:`then`
          (bind (_color_2 _secondary_color_2 _display_name_2 _description_2) (break `/Game/Neurorama/InfoActors/Sia_Array` _returnvalue_4))
          ;[1 1 1] Duplicated InfoActors and Single-Instance InfoActors
          ;;[1 1 1] Set colors
          (`MeshComponent.SetVectorParameterValueOnMaterials` (`self.InfoActMesh`) "PrimaryColor" (`KismetMathLibrary.Conv_LinearColorToVector` (`KismetStringLibrary.Conv_StringToColor` _color_2))) ; Functionality: any vector with name "PrimaryColor" in a material blueprint will be colored..
          (`MeshComponent.SetVectorParameterValueOnMaterials` (`self.InfoActMesh`) "SecondaryColor" (`KismetMathLibrary.Conv_LinearColorToVector` (`KismetStringLibrary.Conv_StringToColor` _secondary_color_2)))
          ;;[1 1 1] Set InfoActor name and description
          (set `self.Name` (`KismetTextLibrary.Conv_StringToText` _display_name_2))
          (set `self.Description` (`KismetTextLibrary.Conv_StringToText` _description_2)))
        (:`RowNotFound`
          (`KismetSystemLibrary.PrintString` _returnvalue true true (struct :`R` 1.0 :`B` 0.080132 :`A` 1.0) 15.0) ; print out missing infoActor references
        )))))