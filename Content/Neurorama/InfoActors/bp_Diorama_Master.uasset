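; Master diorama actor that manages gaze hover and selection of info actors in the Neurorama game.
; Registers itself with the Game Instance at BeginPlay and uses its collected info actor list to clear hover or selection.
; Hovering or selecting sends messages to every actor of the target's class, so matching parts highlight together.
; Selection toggles on a repeated class, plays a sound and returns name and description for the HUD.
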(event `self.ReceiveBeginPlay`
  ;[0 0.3916 0.8879] At begin play, add all dioramas to an array in the Game Instance
  (bind _asbp_game_instance (cast `/Game/Neurorama/Core/BP_GameInstance` (`GameplayStatics.GetGameInstance`)))
  (`KismetArrayLibrary.Array_Add` (`/Game/Neurorama/Core/BP_GameInstance.dioramasCollected` _asbp_game_instance) self))

(fn `deselectAllInfoActors`
  (bind _asbp_game_instance (cast `/Game/Neurorama/Core/BP_GameInstance` (`GameplayStatics.GetGameInstance`)))
  (for _array_element (`/Game/Neurorama/Core/BP_GameInstance.infoActorsCollected` _asbp_game_instance)
    (message `/Game/Neurorama/InfoActors/BPI_infoInterfaces.DisengageInfoActor` _array_element))
  (return))

(fn `hoverOverInfoActor`
  (params (infoActorReference :type "Actor Object Reference"))
  (returns (Name :type Text))
  (cast `/Game/Neurorama/InfoActors/BP_ia_Master` infoActorReference
    (:`then`
      ;[0 0.3968 0.9047] Is infoActor already selected?
      (if (== (`GameplayStatics.GetObjectClass` infoActorReference) (`GameplayStatics.GetObjectClass` (`self.hoveredInfoActor`)))
        _
        (else
          (`self.unhoverAllInfoActors`)
          (bind _outactors (`GameplayStatics.GetAllActorsOfClass` (`GameplayStatics.GetObjectClass` infoActorReference)))
          (for _array_element _outactors
            (message `/Game/Neurorama/InfoActors/BPI_infoInterfaces.gazeHover` _array_element))
          (bind _output_get (set `self.hoveredInfoActor` infoActorReference))
          (bind _asbp_ia_master (cast `/Game/Neurorama/InfoActors/BP_ia_Master` _output_get))
          (return (`/Game/Neurorama/InfoActors/BP_ia_Master.Name` _asbp_ia_master)))))
    (:`CastFailed`
      ;[1 1 1] If BPia test fails
      (`self.unhoverAllInfoActors`)))
  (set `self.hoveredInfoActor` "/Game/Neurorama/InfoActors/BP_ia_Master.BP_ia_Master")
  (return ""))

(fn `selectInfoActor`
  (params (`infoActor Location` :type "Vector Structure") (`infoActor Reference` :type "Actor Object Reference"))
  (returns (isDeselectingAll :type Boolean) (Name :type Text) (Description :type Text) (SpecialDescription :type Text))
  (cast `/Game/Neurorama/InfoActors/BP_ia_Master` `infoActor Reference`
    (:`then`
      (`self.deselectAllInfoActors`) ; If player selects an infoActor, first pre-emtively deselect all infoActors
      ;[0 0.3968 0.8963] Test to see if player has selected and already-selected infoActor. If so, it was deselected in the last step so we're all set. If it's a new infoActor, we'll select it in the next step.
      (if (== (`GameplayStatics.GetObjectClass` (`self.selectedInfoActor`)) (`GameplayStatics.GetObjectClass` `infoActor Reference`))
        ;[0.1384 0.3712 0.02956] Code to play SFX
        (`GameplayStatics.PlaySoundAtLocation` null `infoActor Location`)
        (else
          ;[0.09306 0.000304 0.4564] If player selects an unselected infoActor, select it, and any other infoActors of the same class
          (bind _outactors (`GameplayStatics.GetAllActorsOfClass` (`GameplayStatics.GetObjectClass` `infoActor Reference`)))
          (for _array_element _outactors
            (message `/Game/Neurorama/InfoActors/BPI_infoInterfaces.EngageInfoActor` _array_element))
          (`GameplayStatics.PlaySoundAtLocation` null `infoActor Location`)
          (bind _output_get (set `self.selectedInfoActor` `infoActor Reference`))
          (bind _asbp_ia_master (cast `/Game/Neurorama/InfoActors/BP_ia_Master` _output_get))
          ;[0.1812 0.006512 0.2789] Return to update HUD, etc
          (return false (`/Game/Neurorama/InfoActors/BP_ia_Master.Name` _asbp_ia_master) (`/Game/Neurorama/InfoActors/BP_ia_Master.Description` _asbp_ia_master) ""))))
    (:`CastFailed`
      (`self.deselectAllInfoActors`) ; If player presses select button with no infoActor in view, deselect all infoActors
      (`GameplayStatics.PlaySound2D` null 0.01)))
  (set `self.selectedInfoActor` "/Game/Neurorama/InfoActors/BP_ia_Master.BP_ia_Master") ; reset selected infoActor to master, which is default
  (return true "" "" ""))

(fn `unhoverAllInfoActors`
  (bind _asbp_game_instance (cast `/Game/Neurorama/Core/BP_GameInstance` (`GameplayStatics.GetGameInstance`)))
  (for _array_element (`/Game/Neurorama/Core/BP_GameInstance.infoActorsCollected` _asbp_game_instance)
    (message `/Game/Neurorama/InfoActors/BPI_infoInterfaces.gazeIgnore` _array_element))
  (return))

(fn `UserConstructionScript`)