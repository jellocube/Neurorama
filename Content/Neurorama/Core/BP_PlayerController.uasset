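; Player controller for Neurorama's brain model that cycles anatomical display modes on Space or a motion-controller face button, starting with everything visible.
; NextDisplayMode switches on DisModeId through half-cortex, interior, limbic, midbrain/brainstem and complete views.
; A macro iterates the GameInstance's InfoActor list, hiding or revealing each by region or hemisphere grouping, then the mode title flashes briefly.
; LastDisplayMode and EnterMenu are empty stubs.
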(event `Key|SpaceBar`
  (params (Key :type "Key Structure"))
  ;[1 1 1] Display mode controls & switch
  (:`Pressed`
    (`self.nextDisplayMode` :!label _label)))

(event `Key|MotionController_Right_FaceButton1`
  (params (Key :type "Key Structure"))
  ;[1 1 1] Display mode controls & switch
  (:`Released`
    (goto _label)))

(event `nextDisplayMode`
  ;[1 1 1] Display mode controls & switch
  (switch `int` (`self.disModeId`)
    (:`Default`
      (`KismetSystemLibrary.PrintString` "Displaying: left cortex + interior" :!label _label_2)
      (set `self.disModeName` "Half-Cortex Displaying")
      ;[1 1 1] Hide all right-handed infoActors in cortices
      (bind _array_element (`self.Iterate through all infoActors in play`)
        (:`LoopBody`
          (bind _asbp_info_actor_master (cast `/Game/Neurorama/Core/BP_infoActor_Master` _array_element))
          (bind _isincortex (`/Game/Neurorama/Core/BP_infoActor_Master.isInCortex?` _asbp_info_actor_master))
          (if _isincortex
            (if (== (`/Game/Neurorama/Core/BP_infoActor_Master.Grouping` _asbp_info_actor_master) 2)
              (`/Game/Neurorama/Core/BP_infoActor_Master.HideActor` _asbp_info_actor_master)
              ;[0.2935 0.5 0.2425] Add that infoActor to the list of hiddenInfoActors
              (`KismetArrayLibrary.Array_Add` (`self.hiddenInfoActors`) _array_element)
              (else
                (`/Game/Neurorama/Core/BP_infoActor_Master.Reveal Actor` _asbp_info_actor_master)))))
        (:`Completed`
          (`/Engine/EditorBlueprintResources/StandardMacros.IncrementInt` (`self.disModeId`)
            (:`  `
              (`self.FlashDisplayModeTitle`))))))
    (:`0`
      (`self.Reset variable hiddenInfoActors`)
      (goto _label_2))
    (:`1`
      (`self.Reset variable hiddenInfoActors`)
      (`KismetSystemLibrary.PrintString` "Displaying: interior only")
      (set `self.disModeName` "Inside Structures Displaying")
      ;[1 1 1] Hide all InfoActor children of cortex diorama
      (bind _array_element_2 (`self.Iterate through all infoActors in play`)
        (:`LoopBody`
          (bind _asbp_info_actor_master_2 (cast `/Game/Neurorama/Core/BP_infoActor_Master` _array_element_2))
          (bind _isincortex_2 (`/Game/Neurorama/Core/BP_infoActor_Master.isInCortex?` _asbp_info_actor_master_2))
          (if _isincortex_2
            (`/Game/Neurorama/Core/BP_infoActor_Master.HideActor` _asbp_info_actor_master_2)
            ;[0.2935 0.5 0.2425] Add that infoActor to the list of hiddenInfoActors
            (`KismetArrayLibrary.Array_Add` (`self.hiddenInfoActors`))
            (else
              (`/Game/Neurorama/Core/BP_infoActor_Master.Reveal Actor` _asbp_info_actor_master_2))))
        (:`Completed`
          (`/Engine/EditorBlueprintResources/StandardMacros.IncrementInt` (`self.disModeId`)
            (:`  `
              (`self.FlashDisplayModeTitle`))))))
    (:`2`
      (`self.Reset variable hiddenInfoActors`)
      (`KismetSystemLibrary.PrintString` "Displaying: limbic system only")
      (set `self.disModeName` "Limbic System Displaying")
      ;[1 1 1] Show only Limbic system
      (bind _array_element_3 (`self.Iterate through all infoActors in play`)
        (:`LoopBody`
          (bind _asbp_info_actor_master_3 (cast `/Game/Neurorama/Core/BP_infoActor_Master` _array_element_3))
          (bind _isinlimbic (`/Game/Neurorama/Core/BP_infoActor_Master.isInLimbic?` _asbp_info_actor_master_3))
          (if _isinlimbic
            (`/Game/Neurorama/Core/BP_infoActor_Master.Reveal Actor` _asbp_info_actor_master_3)
            (else
              (`/Game/Neurorama/Core/BP_infoActor_Master.HideActor` _asbp_info_actor_master_3))))
        (:`Completed`
          (`/Engine/EditorBlueprintResources/StandardMacros.IncrementInt` (`self.disModeId`)
            (:`  `
              (`self.FlashDisplayModeTitle`))))))
    (:`3`
      (`self.Reset variable hiddenInfoActors`)
      (`KismetSystemLibrary.PrintString` "Displaying: midbrain and brainstems only")
      (set `self.disModeName` "Midbrain & Brainstem Displaying")
      ;[1 1 1] Show only Limbic system
      (bind _array_element_4 (`self.Iterate through all infoActors in play`)
        (:`LoopBody`
          (bind _asbp_info_actor_master_4 (cast `/Game/Neurorama/Core/BP_infoActor_Master` _array_element_4))
          (bind _isinbrainstem (`/Game/Neurorama/Core/BP_infoActor_Master.isInBrainstem?` _asbp_info_actor_master_4))
          (if _isinbrainstem
            (`/Game/Neurorama/Core/BP_infoActor_Master.Reveal Actor` _asbp_info_actor_master_4)
            (else
              (`/Game/Neurorama/Core/BP_infoActor_Master.HideActor` _asbp_info_actor_master_4))))
        (:`Completed`
          (`/Engine/EditorBlueprintResources/StandardMacros.IncrementInt` (`self.disModeId`)
            (:`  `
              (`self.FlashDisplayModeTitle`))))))
    (:`4`
      (`self.Reset variable hiddenInfoActors` :!label _label_3)
      (`KismetSystemLibrary.PrintString` "Diplaying All")
      (set `self.disModeName` "Complete Display")
      ;[1 1 1] Reveal all infoActors
      (bind _array_element_5 (`self.Iterate through all infoActors in play`)
        (:`LoopBody`
          (bind _asbp_info_actor_master_5 (cast `/Game/Neurorama/Core/BP_infoActor_Master` _array_element_5))
          (`/Game/Neurorama/Core/BP_infoActor_Master.Reveal Actor` _asbp_info_actor_master_5))
        (:`Completed`
          (set `self.disModeId` 0)
          (`self.FlashDisplayModeTitle`))))))

(event `lastDisplayMode`
  ;[1 1 1] Display mode controls & switch
)

(event `self.ReceiveBeginPlay`
  (goto _label_3))

(fn `EnterMenu`
  (returns (ExitedMenu :type Boolean)))

(fn `UserConstructionScript`)