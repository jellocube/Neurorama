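; Main menu pawn that adds the desktop walk HUD and main menu widgets to the viewport on BeginPlay.
; It also defines helper graphs to hover, select, unhover and deselect InfoActors, though its event graph calls none of them.
; Hover and select are delegated to the InfoActor's parent BP_Diorama_Master.
; Unhover and deselect target the dioramas collected in BP_GameInstance.
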(event `self.ReceiveBeginPlay`
  ;[1 1 1] Event BeginPlay
  (bind _returnvalue (`|CreateWidget` "/Game/Neurorama/Core/W_Desktop_WalkHUD.W_Desktop_WalkHUD_C"))
  (`UserWidget.AddToViewport` _returnvalue 0)
  (bind _returnvalue_2 (`|CreateWidget` "/Game/Neurorama/Widgets/W_MainMenu.W_MainMenu_C" (`GameplayStatics.GetPlayerController` 0)))
  (`UserWidget.AddToViewport` _returnvalue_2 0))

(fn `UserConstructionScript`)