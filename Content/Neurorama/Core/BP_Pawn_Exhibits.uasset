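; Player pawn for exhibits that creates HUD and controls widgets, toggles the main menu, and handles pointer interaction with dioramas.
; Tick traces under the cursor to set the highlighted infoactor and rotates the current diorama when a touch drag passes a small threshold.
; Touch release toggles that infoactor's selection through its parent diorama or deselects across collected dioramas.
; Selection name and description text is written to the player controller.
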(event `self.ReceiveBeginPlay`
  ;[1 1 1] Event BeginPlay
  (bind _returnvalue (`|CreateWidget` "/Game/Neurorama/Core/W_Desktop_WalkHUD.W_Desktop_WalkHUD_C"))
  (`UserWidget.AddToViewport` _returnvalue 0)
  (bind _returnvalue_2 (`|CreateWidget` "/Game/Neurorama/Widgets/W_Controls_Exhibit.W_Controls_Exhibit_C" (`GameplayStatics.GetPlayerController` 0)))
  (`UserWidget.AddToViewport` _returnvalue_2 0))

(event `InputAction|Finger 1`
  (params (Key :type "Key Structure"))
  (bind _highlightedinfoactor (`self.HighlightedInfoactor`))
  (:`Pressed`
    (set `self.Finger 1 Pressed` true)
    (set `self.Touch Start Position` (`self.Get Finger Position` "Touch1")))
  (:`Released`
    (set `self.Finger 1 Pressed` false)
    ;[0.003347 0.3968 0.8632] Selection code
    (cast `/Game/Neurorama/Core/InfoActors/BP_infoActor_Master` _highlightedinfoactor ; Was the object selected an infoActor?
      (:`then`
        (bind (_infoactor_name _infoactor_description) (`self.Select Infoactor` _highlightedinfoactor)
          (:`Was Unselected`
            ;;[0.807 0.2016 0.402] Wipe display text
            (bind _asbp_player_controller (cast `/Game/Neurorama/Core/BP_PlayerController` (`GameplayStatics.GetPlayerController` 0) :!label _label))
            (set `/Game/Neurorama/Core/BP_PlayerController.CurrentSelectionName` "" _asbp_player_controller)
            (set `/Game/Neurorama/Core/BP_PlayerController.CurrentSelectionDescription` "" _asbp_player_controller))
          (:`Was Selected`
            ;;[0.807 0.2016 0.402] Assign display text
            (bind _asbp_player_controller_2 (cast `/Game/Neurorama/Core/BP_PlayerController` (`GameplayStatics.GetPlayerController` 0)))
            (set `/Game/Neurorama/Core/BP_PlayerController.CurrentSelectionName` _infoactor_name _asbp_player_controller_2)
            (set `/Game/Neurorama/Core/BP_PlayerController.CurrentSelectionDescription` _infoactor_description _asbp_player_controller_2))))
      (:`CastFailed`
        (`self.Deselect Infoactors in all Dioramas`) ; If player clicks on something not an infoActor (i.e., the background) , tell all dioramas to deselct all infoActors
        ;;[0.3281 0.6761 1] if something was selected before (i.e., a deselection occured), play unpopping sound
        (if (`KismetTextLibrary.TextIsEmpty` (`self.SelectionName`))
          (goto _label)
          (else
            (`GameplayStatics.CreateSound2D` "/Game/Neurorama/SFX/A_SelectNot01.A_SelectNot01" 1.0 1.0 0.0 null)
            (goto _label)))))))

(event `Key|Escape`
  (params (Key :type "Key Structure"))
  ;[1 0.3804 0.8471] Code to show main menu
  (:`Pressed`
    (if (`self.MainMenuIsOpen`) :!label _label_2
      (bind _foundwidgets (`WidgetBlueprintLibrary.GetAllWidgetsOfClass` "/Game/Neurorama/Widgets/W_MainMenu.W_MainMenu_C" false))
      (`Widget.RemoveFromParent` _foundwidgets)
      (set `self.MainMenuIsOpen` false)
      (else
        (bind _returnvalue (`|CreateWidget` "/Game/Neurorama/Widgets/W_MainMenu.W_MainMenu_C" (`GameplayStatics.GetPlayerController` 0)))
        (`UserWidget.AddToViewport` _returnvalue 0)
        (set `self.MainMenuIsOpen` true)))))

(event `Key|O`
  (params (Key :type "Key Structure"))
  ;[1 0.3804 0.8471] Code to show main menu
  (:`Pressed`
    (goto _label_2)))

(event `OpenMainMenu`
  ;[1 0.3804 0.8471] Code to show main menu
  (goto _label_2))

(event `self.ReceiveTick`
  (params (DeltaSeconds :type "Float (single-precision)"))
  (bind (_touch_start_position_x _touch_start_position_y) (`KismetMathLibrary.BreakVector2D` (`self.Touch Start Position`)))
  (bind (_touch_last_known_position_x _touch_last_known_position_y) (`KismetMathLibrary.BreakVector2D` (`self.Touch Last Known Position`)))
  (bind _sizex (`PlayerController.GetViewportSize` (`GameplayStatics.GetPlayerController` 0)))
  (`|ExecutionSequence`
    (:`then_0`
      ;[0.003347 0.3968 0.8632] Hover code
      (bind _asbp_info_actor_master (cast `/Game/Neurorama/Core/InfoActors/BP_infoActor_Master` (`.HitActor` (`GameplayStatics.BreakHitResult` (`PlayerController.GetHitResultUnderCursorByChannel` (`GameplayStatics.GetPlayerController` 0) "TraceTypeQuery1" true)))) ; Was the object selected an infoActor?
        (:`then`
          (`self.Hover Over Infoactor` _asbp_info_actor_master
            (:`exec`
              _)))
        (:`CastFailed`
          (`self.Unhover Infoactors in all Dioramas` :!label _label_3
            (:`exec`
              _))))
      (set `self.HighlightedInfoactor` _asbp_info_actor_master))
    (:`then_1`
      (if (`self.Finger 1 Pressed`)
        (if (> (`KismetMathLibrary.VSize2D` (- (`self.Touch Start Position`) (`self.Get Finger Position` "Touch1"))) 5.0)
          (set `self.Touch Last Known Position` (`self.Get Finger Position` "Touch1"))
          (bind _asbp_state (cast `/Game/Neurorama/Core/BP_State` (`GameplayStatics.GetGameState`)))
          (`/Game/Neurorama/Core/InfoActors/BP_Diorama_Master.AddRotation` (`/Game/Neurorama/Core/BP_State.CurrentDiorama` _asbp_state) (`KismetMathLibrary.MakeVector2D` (/ (- _touch_start_position_x _touch_last_known_position_x) (`KismetMathLibrary.Conv_IntToDouble` _sizex)) (/ (- _touch_start_position_y _touch_last_known_position_y) (`KismetMathLibrary.Conv_IntToDouble` _sizex)))))))))

(event `Key|E`
  (params (Key :type "Key Structure"))
  ;[0.003347 0.3968 0.8632] Hover code
  (:`Released`
    (goto _label_3)))

(fn `UserConstructionScript`)