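; Master actor for selectable brain-structure models in Neurorama, each carrying a display name and description.
; Construction looks up IndexName in DT_iaData to set material colors and text, while functions query the same row for cortex, limbic and brainstem membership.
; BeginPlay registers the actor in the Game Instance's InfoActorsCollected array.
; Reversible timelines drive material parameters for selection, gaze hover and hide/reveal, which also toggles collision so hidden actors ignore selection.
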(event `self.ReceiveBeginPlay`
  ;[0 0.6654 1] At begin play, add all infoActors to an array in the Game Instance
  (bind _asbp_game_instance (cast `/Game/Neurorama/Core/BP_GameInstance` (`GameplayStatics.GetGameInstance`)))
  (`KismetArrayLibrary.Array_Add` (`/Game/Neurorama/Core/BP_GameInstance.infoActorsCollected` _asbp_game_instance) self)
  (`PrimitiveComponent.SetCollisionEnabled` (`self.InfoActMesh`) "QueryAndPhysics") ; enable collision, since apparently the objects don't start with it on if they're not visible (?)
)

(event `/Game/Neurorama/Core/BPI_infoInterfaces.EngageInfoActor`
  ;[0.235 0.03525 0.06854] Code to highlight infoActors when engaged (clicked)/disengaged (clicked off)
  (bind (_direction _gotcurvescurve) (`Timeline|selectionHighlight` :!label _label)
    (:`Update`
      (`MeshComponent.SetScalarParameterValueOnMaterials` (`self.InfoActMesh`) "selectValue" (`KismetMathLibrary.Lerp` 0.0 (`self.HighlightIntensity`) _gotcurvescurve)))))

(event `/Game/Neurorama/Core/BPI_infoInterfaces.DisengageInfoActor`
  ;[0.235 0.03525 0.06854] Code to highlight infoActors when engaged (clicked)/disengaged (clicked off)
  (goto _label :!via `Reverse`))

(event `/Game/Neurorama/Core/BPI_infoInterfaces.gazeHover`
  ;[0.235 0.03525 0.06854] Code to hoverhighlight objects when gazed upon/ignored
  (bind (_direction _linearrise) (`Timeline|hoverHighlight` :!label _label_2)
    (:`Update`
      (`MeshComponent.SetScalarParameterValueOnMaterials` (`self.InfoActMesh`) "hoverValue" (`KismetMathLibrary.Lerp` 0.0 (`self.HoverIntensity`) _linearrise)))))

(event `/Game/Neurorama/Core/BPI_infoInterfaces.gazeIgnore`
  ;[0.235 0.03525 0.06854] Code to hoverhighlight objects when gazed upon/ignored
  (goto _label_2 :!via `Reverse`))

(event `HideActor`
  (bind _infoactmesh (`self.InfoActMesh`))
  ;[0 0.8632 0.5737] Code to hide objects for displaying different models
  ;;[1 1 1] By disabling collision, mouse and motion controller selection won't affect hidden actors
  (`PrimitiveComponent.SetCollisionEnabled` (`self.InfoActMesh`) "NoCollision")
  (bind (_direction _visibilityrevealetccurve _fresnelcurve) (`Timeline|changeOpacity` :!label _label_3)
    (:`Update`
      (`MeshComponent.SetScalarParameterValueOnMaterials` _infoactmesh "BaseOpacity" (`KismetMathLibrary.Lerp` 0.02 (`self.defaultOpacity`) _visibilityrevealetccurve))
      (`MeshComponent.SetScalarParameterValueOnMaterials` _infoactmesh "FresnelLerp" (`KismetMathLibrary.Lerp` 0.0 1.0 _fresnelcurve)))))

(event `Reveal Actor`
  ;[0 0.8632 0.5737] Code to hide objects for displaying different models
  ;;[1 1 1] By disabling collision, mouse and motion controller selection won't affect hidden actors
  (`PrimitiveComponent.SetCollisionEnabled` (`self.InfoActMesh`) "QueryAndPhysics")
  (goto _label_3 :!via `Reverse`))

(fn `isInBrainstem?`
  (returns (isInBrainstem :type Boolean))
  (bind _indexname (`self.IndexName`))
  (bind _returnvalue (`|GetDataTableRow` "/Game/Neurorama/Core/DT_iaData.DT_iaData" (`KismetStringLibrary.Conv_StringToName` _indexname))
    (:`then`
      (return (`.inBrainstem_77_319670C448CB32D83E88BF9738CC7878` (break `/Game/Neurorama/Core/S_iaStructure` _returnvalue))))
    (:`RowNotFound`
      (`KismetSystemLibrary.PrintString` _indexname true true (struct :`R` 1.0 :`B` 0.125939 :`A` 1.0)))))

(fn `isInCortex?`
  (returns (isInCortex :type Boolean))
  (bind _indexname (`self.IndexName`))
  (bind _returnvalue (`|GetDataTableRow` "/Game/Neurorama/Core/DT_iaData.DT_iaData" (`KismetStringLibrary.Conv_StringToName` _indexname)) ; This table contains all of the InfoActor  information.
    (:`then`
      (return (`.inCortex_73_ADDBA0834AC7E5F9B60C3FA92FAFBE11` (break `/Game/Neurorama/Core/S_iaStructure` _returnvalue))))
    (:`RowNotFound`
      (`KismetSystemLibrary.PrintString` _indexname true true (struct :`R` 1.0 :`B` 0.125939 :`A` 1.0)))))

(fn `isInLimbic?`
  (returns (isInLimbic :type Boolean))
  (bind _indexname (`self.IndexName`))
  (bind _returnvalue (`|GetDataTableRow` "/Game/Neurorama/Core/DT_iaData.DT_iaData" (`KismetStringLibrary.Conv_StringToName` _indexname)) ; This table contains all of the InfoActor  information.
    (:`then`
      (return (`.inLimbic_75_7DD54139430213625D17A3B61653A0FF` (break `/Game/Neurorama/Core/S_iaStructure` _returnvalue))))
    (:`RowNotFound`
      (`KismetSystemLibrary.PrintString` _indexname true true (struct :`R` 1.0 :`B` 0.125939 :`A` 1.0)))))

(fn `UserConstructionScript`
  (locals (NewLocalVar_0 :type "Material Object Reference"))
  (bind _indexname (`self.IndexName`))
  (bind _indexname_2 (`self.IndexName`))
  ;[1 1 1] Create dynamic material instance(s)
  (`KismetMaterialLibrary.CreateDynamicMaterialInstance` (`PrimitiveComponent.GetMaterial` (`self.InfoActMesh`) 0))
  ;[1 1 1] Look up infoActor color in CSV datatable
  (if (== (`self.Grouping`) 0)
    (bind _returnvalue (`|GetDataTableRow` "/Game/Neurorama/Core/DT_iaData.DT_iaData" (`KismetStringLibrary.Conv_StringToName` _indexname_2))
      (:`then`
        (bind (_color1 _color2 _fleshcolor1 _fleshcolor2 _display_name _description) (break `/Game/Neurorama/Core/S_iaStructure` _returnvalue))
        ;[1 1 1] Duplicated InfoActors and Single-Instance InfoActors
        ;;[1 1 1] Set colors
        (`MeshComponent.SetVectorParameterValueOnMaterials` (`self.InfoActMesh`) "PrimaryColor" (`KismetMathLibrary.Conv_LinearColorToVector` (`KismetStringLibrary.Conv_StringToColor` _color1))) ; Functionality: any vector with name "PrimaryColor" in a material blueprint will be colored..
        (`MeshComponent.SetVectorParameterValueOnMaterials` (`self.InfoActMesh`) "SecondaryColor" (`KismetMathLibrary.Conv_LinearColorToVector` (`KismetStringLibrary.Conv_StringToColor` _color2)))
        ;;[1 1 1] Set Opacity
        (`MeshComponent.SetVectorParameterValueOnMaterials` (`self.InfoActMesh`) "BaseOpacity" (`KismetMathLibrary.Conv_DoubleToVector` (`self.defaultOpacity`)))
        ;;[1 1 1] Set InfoActor name and description
        (set `self.DisplayName` (`KismetTextLibrary.Conv_StringToText` _display_name))
        (set `self.DisplayDescription` (`KismetTextLibrary.Conv_StringToText` _description)))
      (:`RowNotFound`
        (`KismetSystemLibrary.PrintString` _indexname_2 true true (struct :`R` 1.0 :`B` 0.080132 :`A` 1.0) 15.0) ; print out missing infoActor references
      ))
    (else
      (bind _returnvalue_2 (`|GetDataTableRow` "/Game/Neurorama/Core/DT_iaData.DT_iaData" (`KismetStringLibrary.Conv_StringToName` _indexname))
        (:`then`
          (bind (_color1_2 _color2_2 _fleshcolor1_2 _fleshcolor2_2 _display_name_2 _description_2) (break `/Game/Neurorama/Core/S_iaStructure` _returnvalue_2))
          ;[1 1 1] InfoActors with asymmetrical mesh pairs
          ;;[1 1 1] Set colors
          (`MeshComponent.SetVectorParameterValueOnMaterials` (`self.InfoActMesh`) "PrimaryColor" (`KismetMathLibrary.Conv_LinearColorToVector` (`KismetStringLibrary.Conv_StringToColor` _color1_2))) ; Functionality: any vector with name "PrimaryColor" in a material blueprint will be colored..
          (`MeshComponent.SetVectorParameterValueOnMaterials` (`self.InfoActMesh`) "SecondaryColor" (`KismetMathLibrary.Conv_LinearColorToVector` (`KismetStringLibrary.Conv_StringToColor` _color2_2)))
          ;;[1 1 1] Set Opacity
          (`MeshComponent.SetVectorParameterValueOnMaterials` (`self.InfoActMesh`) "BaseOpacity" (`KismetMathLibrary.Conv_DoubleToVector` (`self.defaultOpacity`)))
          (`MeshComponent.SetVectorParameterValueOnMaterials` (`self.InfoActMesh`) "FresnelLerp" (0.0 0.0 0.0))
          ;;[1 1 1] Set InfoActor name and description
          (set `self.DisplayName` (`KismetTextLibrary.Conv_StringToText` _display_name_2))
          (set `self.DisplayDescription` (`KismetTextLibrary.Conv_StringToText` _description_2)))
        (:`RowNotFound`
          (`KismetSystemLibrary.PrintString` _indexname true true (struct :`R` 0.969136 :`B` 1.0 :`A` 1.0) 15.0) ; print out missing infoActor references
        )))))