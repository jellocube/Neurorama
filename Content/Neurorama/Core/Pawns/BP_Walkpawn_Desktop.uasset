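; Desktop walking pawn for Neurorama, with mouselook and axis movement, used to explore dioramas and inspect their infoActors.
; Cursor traces drive hover on Tick and selection on click, delegating to the owning diorama or clearing all dioramas listed in the GameInstance on a miss.
; Selection stores name and description for display.
; Keys also toggle the main menu, debug-clear hovers, and replace this pawn with a possessed VR pawn.
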(event `Key|V`
  (params (Key :type "Key Structure"))
  ;[0.03525 0.235 0.03525] Testing
  ;;[1 1 1] If player presses V, switch to VR pawn.
  (:`Pressed`
    (bind _returnvalue (`|SpawnActorFromClass` "/Game/Neurorama/Core/Pawns/BP_Walkpawn_VR.BP_Walkpawn_VR_C" (`KismetMathLibrary.MakeTransform` (.location (`SceneComponent.K2_GetComponentToWorld` (`self.FirstPersonCamera`))) (.rotation (`SceneComponent.K2_GetComponentToWorld` (`self.FirstPersonCamera`)))) "Undefined" "OverrideRootScale" null null))
    (`self.SpawnDefaultController` _returnvalue)
    (`Controller.Possess` (`self.GetController`) _returnvalue)
    (`KismetSystemLibrary.PrintString` "possessed VR pawn")
    (`self.K2_DestroyActor`)))

(event `InputAxis|LookUp`
  (params (AxisValue :type "Float (single-precision)"))
  ;[0.235 0.03525 0.06854] Movement Input, etc.
  ;;[1 1 1] Movement and mouselook code
  ;;;[1 1 1] Look Control
  (`self.AddControllerPitchInput` AxisValue))

(event `InputAxis|Turn`
  (params (AxisValue :type "Float (single-precision)"))
  ;[0.235 0.03525 0.06854] Movement Input, etc.
  ;;[1 1 1] Movement and mouselook code
  ;;;[1 1 1] Look Control
  (`self.AddControllerYawInput` AxisValue))

(event `InputAxis|MoveForward`
  (params (AxisValue :type "Float (single-precision)"))
  ;[0.235 0.03525 0.06854] Movement Input, etc.
  ;;[1 1 1] Movement and mouselook code
  ;;;[1 1 1] Movement input basic
  (`self.AddMovementInput` (`KismetMathLibrary.GetForwardVector` (`KismetMathLibrary.MakeRotator` 0.0 (.pitch (`self.GetControlRotation`)) (.yaw (`self.GetControlRotation`)))) (* AxisValue 0.7)))

(event `InputAxis|MoveRight`
  (params (AxisValue :type "Float (single-precision)"))
  ;[0.235 0.03525 0.06854] Movement Input, etc.
  ;;[1 1 1] Movement and mouselook code
  ;;;[1 1 1] Movement input basic
  (`self.AddMovementInput` (`KismetMathLibrary.GetRightVector` (`KismetMathLibrary.MakeRotator` 0.0 (.pitch (`self.GetControlRotation`)) (.yaw (`self.GetControlRotation`)))) AxisValue))

(event `self.ReceiveTick`
  (params (DeltaSeconds :type "Float (single-precision)"))
  (bind (_bblockinghit _binitialoverlap _time _distance _location _impactpoint _normal _impactnormal _physmat _hitactor) (`GameplayStatics.BreakHitResult` (`PlayerController.GetHitResultUnderCursorByChannel` (`GameplayStatics.GetPlayerController` 0) "TraceTypeQuery1" true)))
  ;[0.003347 0.3968 0.8632] Hover code
  ;;[0.1746 0.006512 0.006512] Mouse hover over infoActor code
  (`self.isPawnControlled?`)
  (bind _asbp_info_actor_master (cast `/Game/Neurorama/Core/BP_infoActor_Master` _hitactor) ; Was the object selected an infoActor?
    (:`then`
      ;;[0.07819 0.1845 0.2831] Tell Diorama that owns hit object to select it if it is an infoActor
      (bind _asbp_diorama_master (cast `/Game/Neurorama/Core/bp_Diorama_Master` (`self.GetParentActor` _hitactor))) ; Cast to diorama which owns the infoActor, because dioramas contain a lot of the UX/UI code for infoActor display methods, just to keep things organized
      (`/Game/Neurorama/Core/bp_Diorama_Master.hoverOverInfoActor` _asbp_diorama_master _asbp_info_actor_master))
    (:`CastFailed`
      ;;[0 0.3864 0.8796] If player hovers over something not an infoActor (i.e., the background) , tell all dioramas to unhover all infoActors
      (bind _asbp_game_instance (cast `/Game/Neurorama/Core/BP_GameInstance` (`GameplayStatics.GetGameInstance`) :!label _label))
      (for _array_element (`/Game/Neurorama/Core/BP_GameInstance.dioramasCollected` _asbp_game_instance)
        (bind _asbp_diorama_master_2 (cast `/Game/Neurorama/Core/bp_Diorama_Master` _array_element))
        (`/Game/Neurorama/Core/bp_Diorama_Master.unhoverAllInfoActors` _asbp_diorama_master_2)))))

(event `Key|E`
  (params (Key :type "Key Structure"))
  (:`Released`
    (goto _label)))

(event `InputAction|PrimaryButton`
  (params (Key :type "Key Structure"))
  (bind (_bblockinghit _binitialoverlap _time _distance _location _impactpoint _normal _impactnormal _physmat _hitactor) (`GameplayStatics.BreakHitResult` (`PlayerController.GetHitResultUnderCursorByChannel` (`GameplayStatics.GetPlayerController` 0) "TraceTypeQuery1" true)))
  ;[0.003347 0.3968 0.8632] Selection code
  ;;[0.162 0.02029 0.02029] Mouse selecting infoActor code
  (:`Pressed`
    (cast `/Game/Neurorama/Core/BP_infoActor_Master` _hitactor ; Was the object selected an infoActor?
      (:`then`
        ;;[0.0648 0.1651 0.2623] Tell Diorama that owns hit object to select it if it is an infoActor
        (bind _asbp_diorama_master (cast `/Game/Neurorama/Core/bp_Diorama_Master` (`self.GetParentActor` _hitactor)))
        (bind (_isdeselectingall _name _description) (`/Game/Neurorama/Core/bp_Diorama_Master.selectInfoActor` _asbp_diorama_master _location _hitactor))
        (if (== _isdeselectingall true)
          ;;[0.807 0.2016 0.402] Set display text
          (set `self.isSelectedDesc` "" :!label _label_2)
          (set `self.iaSelectedName` "")
          (else
            ;;[0.807 0.2016 0.402] Set display text
            (set `self.isSelectedDesc` _description)
            (set `self.iaSelectedName` _name))))
      (:`CastFailed`
        ;;[0 0.3864 0.8796] If player clicks on something not an infoActor (i.e., the background) , tell all dioramas to deselct all infoActors
        (bind _asbp_game_instance (cast `/Game/Neurorama/Core/BP_GameInstance` (`GameplayStatics.GetGameInstance`)))
        (for _array_element (`/Game/Neurorama/Core/BP_GameInstance.dioramasCollected` _asbp_game_instance)
          (bind _asbp_diorama_master_2 (cast `/Game/Neurorama/Core/bp_Diorama_Master` _array_element))
          (`/Game/Neurorama/Core/bp_Diorama_Master.deselectAllInfoActors` _asbp_diorama_master_2)
          (goto _label_2))))))

(event `Key|Escape`
  (params (Key :type "Key Structure"))
  (:`Pressed`
    (if (`self.menuOpen`) :!label _label_3
      (bind _foundwidgets (`WidgetBlueprintLibrary.GetAllWidgetsOfClass` "/Game/Neurorama/UX/Menus/W_MainMenu.W_MainMenu_C"))
      (`/Game/Neurorama/UX/Menus/W_MainMenu.closeMenu` _foundwidgets)
      (set `self.menuOpen` false)
      (else
        (bind _returnvalue (`|CreateWidget` "/Game/Neurorama/UX/Menus/W_MainMenu.W_MainMenu_C"))
        (`UserWidget.AddToViewport` _returnvalue 0)
        (set `self.menuOpen` true)))))

(event `Key|O`
  (params (Key :type "Key Structure"))
  (:`Pressed`
    (goto _label_3)))

(fn `UserConstructionScript`)