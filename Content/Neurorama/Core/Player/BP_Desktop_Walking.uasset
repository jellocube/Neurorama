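; Desktop player pawn for walking among dioramas and inspecting their info actors with the mouse, with a walk HUD.
; Holding the primary button shows a centered cursor and slows mouselook; cursor traces drive hover, and release toggles selection.
; Parent dioramas handle hover and selection and return display text, while background hits clear every diorama registered in the GameInstance.
; Escape or O toggles the main menu, switching between game-only and UI-only input.
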(event `self.ReceiveBeginPlay`
  (bind _returnvalue (`|CreateWidget` "/Game/Neurorama/Core/Player/W_Desktop_WalkHUD.W_Desktop_WalkHUD_C"))
  (`UserWidget.AddToViewport` _returnvalue 0))

(event `InputAxis|LookUp`
  (params (AxisValue :type "Float (single-precision)"))
  ;[0.235 0.03525 0.06854] Movement Input, etc.
  ;;[1 1 1] Movement and mouselook code
  ;;;[1 1 1] Look Control
  ;;;;[0.3353 0.3596 1] Slow-Motion Mouselook when cursor is shown
  (if (`PlayerController.bShowMouseCursor` (`GameplayStatics.GetPlayerController` 0))
    (`self.AddControllerPitchInput` (* AxisValue 0.2))
    (else
      (`self.AddControllerPitchInput` AxisValue))))

(event `InputAxis|Turn`
  (params (AxisValue :type "Float (single-precision)"))
  ;[0.235 0.03525 0.06854] Movement Input, etc.
  ;;[1 1 1] Movement and mouselook code
  ;;;[1 1 1] Look Control
  ;;;;[0.3353 0.3596 1] Slow-Motion Mouselook when cursor is shown
  (if (`PlayerController.bShowMouseCursor` (`GameplayStatics.GetPlayerController` 0))
    (`self.AddControllerYawInput` (* AxisValue 0.2))
    (else
      (`self.AddControllerYawInput` AxisValue))))

(event `InputAxis|MoveForward`
  (params (AxisValue :type "Float (single-precision)"))
  ;[0.235 0.03525 0.06854] Movement Input, etc.
  ;;[1 1 1] Movement and mouselook code
  ;;;[1 1 1] Movement input basic
  (`self.AddMovementInput` (`KismetMathLibrary.GetForwardVector` (`KismetMathLibrary.MakeRotator` 0.0 (.pitch (`self.GetControlRotation`)) (.yaw (`self.GetControlRotation`)))) (* AxisValue 0.7)))

(event `self.ReceiveTick`
  (params (DeltaSeconds :type "Float (single-precision)"))
  (bind (_bblockinghit _binitialoverlap _time _distance _location _impactpoint _normal _impactnormal _physmat _hitactor) (`GameplayStatics.BreakHitResult` (`PlayerController.GetHitResultUnderCursorByChannel` (`GameplayStatics.GetPlayerController` 0) "TraceTypeQuery1" true)))
  ;[0.003347 0.3968 0.8632] Hover code
  ;;[0.1746 0.006512 0.006512] Mouse hover over infoActor code
  (if (`PlayerController.bShowMouseCursor` (`GameplayStatics.GetPlayerController` 0))
    (`self.isPawnControlled?`
      (:`Return if pawn is controlled`
        (bind _asbp_info_actor_master (cast `/Game/Neurorama/Core/BP_infoActor_Master` _hitactor) ; Was the object selected an infoActor?
          (:`then`
            ;;[0.07819 0.1845 0.2831] Tell Diorama that owns hit object to select it if it is an infoActor
            (bind _asbp_diorama_master (cast `/Game/Neurorama/Core/bp_Diorama_Master` (`self.GetParentActor` _hitactor))) ; Cast to diorama which owns the infoActor, because dioramas contain a lot of the UX/UI code for infoActor display methods, just to keep things organized
            (`/Game/Neurorama/Core/bp_Diorama_Master.HoverOverInfoActor` _asbp_diorama_master _asbp_info_actor_master))
          (:`CastFailed`
            ;;[0 0.3864 0.8796] If player hovers over something not an infoActor (i.e., the background) , tell all dioramas to unhover all infoActors
            (bind _asbp_game_instance (cast `/Game/Neurorama/Core/BP_GameInstance` (`GameplayStatics.GetGameInstance`) :!label _label))
            (for _array_element (`/Game/Neurorama/Core/BP_GameInstance.dioramasCollected` _asbp_game_instance)
              (bind _asbp_diorama_master_2 (cast `/Game/Neurorama/Core/bp_Diorama_Master` _array_element))
              (`/Game/Neurorama/Core/bp_Diorama_Master.UnhoverAllInfoActors` _asbp_diorama_master_2))))))))

(event `InputAxis|MoveRight`
  (params (AxisValue :type "Float (single-precision)"))
  ;[0.235 0.03525 0.06854] Movement Input, etc.
  ;;[1 1 1] Movement and mouselook code
  ;;;[1 1 1] Movement input basic
  (`self.AddMovementInput` (`KismetMathLibrary.GetRightVector` (`KismetMathLibrary.MakeRotator` 0.0 (.pitch (`self.GetControlRotation`)) (.yaw (`self.GetControlRotation`)))) AxisValue))

(event `InputAction|PrimaryButton`
  (params (Key :type "Key Structure"))
  (bind _returnvalue (`GameplayStatics.GetPlayerController` 0))
  ;[0.235 0.03525 0.06854] Movement Input, etc.
  (:`Pressed`
    ;;[0.3353 0.3596 1] Enable mouse cursor on mouse down, and center it. Not activated when Widget has focus
    (set `PlayerController.bShowMouseCursor` true _returnvalue)
    (`self.Center Mouse Cursor` _returnvalue))
  (:`Released`
    (set `PlayerController.bShowMouseCursor` false _returnvalue)
    (`self.AssumeGameMode` _returnvalue)))

(event `Key|E`
  (params (Key :type "Key Structure"))
  (:`Released`
    (goto _label)))

(event `InputAction|PrimaryButton`
  (params (Key :type "Key Structure"))
  (bind (_bblockinghit _binitialoverlap _time _distance _location _impactpoint _normal _impactnormal _physmat _hitactor) (`GameplayStatics.BreakHitResult` (`PlayerController.GetHitResultUnderCursorByChannel` (`GameplayStatics.GetPlayerController` 0) "TraceTypeQuery1" true)))
  ;[0.003347 0.3968 0.8632] Selection code
  ;;[0.162 0.02029 0.02029] Mouse selecting infoActor code
  (:`Released`
    (cast `/Game/Neurorama/Core/BP_infoActor_Master` _hitactor ; Was the object selected an infoActor?
      (:`then`
        ;;[0.0648 0.1651 0.2623] Tell Diorama that owns hit object to select it if it is an infoActor
        (bind _asbp_diorama_master (cast `/Game/Neurorama/Core/bp_Diorama_Master` (`self.GetParentActor` _hitactor)))
        (bind (_unselection_toggled _name _description) (`/Game/Neurorama/Core/bp_Diorama_Master.ToggleInfoActorSelection` _asbp_diorama_master _location _hitactor))
        (if (== _unselection_toggled true)
          ;;[0.807 0.2016 0.402] Wipe display text
          (set `self.SelectionDescription` "" :!label _label_2)
          (set `self.SelectionName` "")
          (else
            ;;[0.807 0.2016 0.402] Assign display text
            (set `self.SelectionDescription` _description)
            (set `self.SelectionName` _name))))
      (:`CastFailed`
        ;;[0 0.3864 0.8796] If player clicks on something not an infoActor (i.e., the background) , tell all dioramas to deselct all infoActors
        (bind _asbp_game_instance (cast `/Game/Neurorama/Core/BP_GameInstance` (`GameplayStatics.GetGameInstance`)))
        (for _array_element (`/Game/Neurorama/Core/BP_GameInstance.dioramasCollected` _asbp_game_instance)
          (bind _asbp_diorama_master_2 (cast `/Game/Neurorama/Core/bp_Diorama_Master` _array_element))
          (`/Game/Neurorama/Core/bp_Diorama_Master.DeselectAllInfoActors` _asbp_diorama_master_2)
          ;;[0.3281 0.6761 1] if something was selected before (i.e., a deselection occured), play unpopping sound
          (if (`KismetTextLibrary.TextIsEmpty` (`self.SelectionName`))
            (goto _label_2)
            (else
              (`GameplayStatics.PlaySoundAtLocation` "/Game/Neurorama/SFX/A_SelectNot01.A_SelectNot01" (`SceneComponent.K2_GetComponentLocation` (`self.Camera`)))
              (goto _label_2))))))))

(event `Key|Escape`
  (params (Key :type "Key Structure"))
  (bind _returnvalue (`GameplayStatics.GetPlayerController` 0))
  ;[1 0.3813 0.8453] Code to show main menu
  (:`Pressed`
    (if (`self.MainMenuIsOpen`) :!label _label_3
      (bind _foundwidgets (`WidgetBlueprintLibrary.GetAllWidgetsOfClass` "/Game/Neurorama/UX/W_MainMenu.W_MainMenu_C" false))
      (`Widget.RemoveFromParent` _foundwidgets)
      (`self.AssumeGameMode` _returnvalue :!label _label_4)
      (else
        (bind _returnvalue_2 (`|CreateWidget` "/Game/Neurorama/UX/W_MainMenu.W_MainMenu_C" _returnvalue))
        (`UserWidget.AddToViewport` _returnvalue_2 0)
        (`self.AssumeMouseMode` _returnvalue _returnvalue_2)))))

(event `Key|O`
  (params (Key :type "Key Structure"))
  ;[1 0.3813 0.8453] Code to show main menu
  (:`Pressed`
    (goto _label_3)))

(event `/Game/Neurorama/Core/Player/BPI_PawnHandler.AssumeGameModeCall`
  ;[1 0.3813 0.8453] Code to show main menu
  (goto _label_4))

(fn `AssumeGameMode`
  (params (Target :type "PlayerController Object Reference"))
  (`WidgetBlueprintLibrary.SetInputMode_GameOnly` Target)
  (`WidgetBlueprintLibrary.SetFocusToGameViewport`)
  (set `PlayerController.bShowMouseCursor` false Target)
  (set `self.MainMenuIsOpen` false)
  (return))

(fn `AssumeMouseMode`
  (params (ThePC :type "PlayerController Object Reference") (FocalWidget :type "Widget Object Reference"))
  (`WidgetBlueprintLibrary.SetInputMode_UIOnlyEx` ThePC FocalWidget)
  (set `PlayerController.bShowMouseCursor` true ThePC)
  (set `self.MainMenuIsOpen` true)
  (`self.Center Mouse Cursor` ThePC)
  (return))

(fn `Center Mouse Cursor`
  (params (ThePC :type "PlayerController Object Reference"))
  (`VictoryBPFunctionLibrary.Viewport__SetMousePosition` ThePC (* (.x (`KismetMathLibrary.Conv_Vector2DToVector` (`WidgetLayoutLibrary.GetViewportSize`) 1.0)) 0.5) (* (.y (`KismetMathLibrary.Conv_Vector2DToVector` (`WidgetLayoutLibrary.GetViewportSize`) 1.0)) 0.5)))

(fn `UserConstructionScript`)