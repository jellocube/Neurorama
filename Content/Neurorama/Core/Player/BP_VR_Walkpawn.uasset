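; BP_VR_Walkpawn is the VR walking pawn, moving relative to camera yaw and using a motion-controller laser pointer to inspect infoActors inside dioramas.
; Each tick, line traces position the laser beam and impact and drive hover highlighting through the owning diorama.
; The primary button selects the pointed infoActor and shows its name and description as HUD text, or deselects everything across all GameInstance dioramas.
; Pressing V swaps to a newly spawned desktop pawn.
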(event `Key|V`
  (params (Key :type "Key Structure"))
  ;[1 1 1] If player presses V, switch to desktop pawn.
  (:`Pressed`
    (bind _returnvalue (`|SpawnActorFromClass` "/Game/Neurorama/Core/Player/BP_Desktop_Walking.BP_Desktop_Walking_C" (`KismetMathLibrary.MakeTransform` (.location (`SceneComponent.K2_GetComponentToWorld` (`self.Camera`))) (.rotation (`SceneComponent.K2_GetComponentToWorld` (`self.Camera`)))) "Undefined" "OverrideRootScale" null null))
    (`self.SpawnDefaultController` _returnvalue)
    (`Controller.Possess` (`self.GetController`) _returnvalue)
    (`KismetSystemLibrary.PrintString` "possessed desktop pawn")
    (`self.K2_DestroyActor`)))

(event `InputAxis|MoveForward`
  (params (AxisValue :type "Float (single-precision)"))
  ;[0.05448 0.1441 0.2307] Movement input basic
  (`self.AddMovementInput` (`KismetMathLibrary.GetForwardVector` (`KismetMathLibrary.MakeRotator` 0.0 0.0 (.yaw (`SceneComponent.RelativeRotation` (`self.Camera`))))) (* AxisValue -0.1)))

(event `InputAxis|MoveRight`
  (params (AxisValue :type "Float (single-precision)"))
  ;[0.05448 0.1441 0.2307] Movement input basic
  (`self.AddMovementInput` (`KismetMathLibrary.GetRightVector` (`KismetMathLibrary.MakeRotator` 0.0 0.0 (.yaw (`SceneComponent.RelativeRotation` (`self.Camera`))))) (* AxisValue 0.1)))

(event `InputAction|PrimaryButton`
  (params (Key :type "Key Structure"))
  (bind _mocon_r_arrow (`self.MoCon_R_Arrow`))
  (bind _returnvalue (`SceneComponent.K2_GetComponentLocation` _mocon_r_arrow))
  ;[1 1 1] Laserpointer BP_IA selection code
  ;;[0.1746 0.006512 0.006512] Click-to-select infoActor code
  (:`Pressed`
    (`self.isPawnControlled?`)
    (bind _asbp_player_controller (cast `/Game/Neurorama/Core/Player/BP_PlayerController` (`GameplayStatics.GetPlayerController` 0)))
    (bind _outhit (`KismetSystemLibrary.LineTraceSingle` _returnvalue (+ _returnvalue (* (`SceneComponent.GetForwardVector` _mocon_r_arrow) 1000000.0)) "TraceTypeQuery1" true))
    (bind (_bblockinghit _binitialoverlap _time _distance _location _impactpoint _normal _impactnormal _physmat _hitactor) (`GameplayStatics.BreakHitResult` _outhit))
    (bind _asbp_info_actor_master (cast `/Game/Neurorama/Core/BP_infoActor_Master` _hitactor)
      (:`then`
        ;;[0.0648 0.1651 0.2623] Tell Diorama that owns hit object to select it if it is an infoActor
        (bind _asbp_diorama_master (cast `/Game/Neurorama/Core/bp_Diorama_Master` (`self.GetParentActor` _asbp_info_actor_master)))
        (bind (_isdeselectingall _name _description) (`/Game/Neurorama/Core/bp_Diorama_Master.selectInfoActor` _asbp_diorama_master _location _asbp_info_actor_master))
        (if (not (== _isdeselectingall true))
          ;;[0.7379 0.1912 0.3712] Update HUD Information
          (`TextRenderComponent.K2_SetText` (`self.textTitle`) _name)
          (`SceneComponent.SetVisibility` (`self.textTitle`) true false)
          (`TextRenderComponent.K2_SetText` (`self.textSubtitle`) _description)
          (`SceneComponent.SetVisibility` (`self.textSubtitle`) true false)))
      (:`CastFailed`
        ;;[0 0.3864 0.8796] If player clicks on something not an infoActor (i.e., the background) , tell all dioramas to deselct all infoActors
        (bind _asbp_game_instance (cast `/Game/Neurorama/Core/BP_GameInstance` (`GameplayStatics.GetGameInstance`)))
        (for _array_element (`/Game/Neurorama/Core/BP_GameInstance.dioramasCollected` _asbp_game_instance)
          (bind _asbp_diorama_master_2 (cast `/Game/Neurorama/Core/bp_Diorama_Master` _array_element))
          (`/Game/Neurorama/Core/bp_Diorama_Master.deselectAllInfoActors` _asbp_diorama_master_2)
          (`SceneComponent.SetVisibility` (`self.textTitle`) false false)
          (`SceneComponent.SetVisibility` (`self.textSubtitle`) false false))))))

(event `self.ReceiveTick`
  (params (DeltaSeconds :type "Float (single-precision)"))
  (bind _mocon_r_arrow (`self.MoCon_R_Arrow`))
  (bind _lasersource (`self.LaserSource`))
  (bind _laserbeam (`self.LaserBeam`))
  (bind _laserimpact (`self.LaserImpact`))
  (bind _returnvalue (`SceneComponent.K2_GetComponentLocation` _lasersource))
  (bind _returnvalue_2 (`SceneComponent.K2_GetComponentLocation` _mocon_r_arrow))
  (bind _returnvalue_3 (+ _returnvalue (* (`SceneComponent.GetForwardVector` _lasersource) 5000.0)))
  (`self.isPawnControlled?`)
  ;[1 1 1] Laser pointer beam code, based on https://www.youtube.com/watch?v=7VaMrs8n8e4&t=12s
  ;;[0.247 0.475 0.2664] Make sure isn't a hidden actor
  (bind _asbp_player_controller (cast `/Game/Neurorama/Core/Player/BP_PlayerController` (`GameplayStatics.GetPlayerController` 0)))
  (bind (_outhit _returnvalue_4) (`KismetSystemLibrary.LineTraceSingle` _returnvalue _returnvalue_3 "TraceTypeQuery1" true))
  (if _returnvalue_4
    (set `self.LaserTargetLoc` (`.Location` (`GameplayStatics.BreakHitResult` _outhit)))
    (else
      (bind _output_get (set `self.LaserTargetLoc` _returnvalue_3))))
  (`ParticleSystemComponent.SetBeamSourcePoint` _laserbeam 0 _returnvalue 0)
  (`ParticleSystemComponent.SetBeamTargetPoint` _laserbeam 0 _output_get 0)
  (`SceneComponent.K2_SetWorldLocation` _laserimpact (- _output_get (`SceneComponent.GetForwardVector` _laserimpact)) false false)
  ;[1 1 1] Laserpointer-based hover-highlighting code
  ;;[0.1441 0.006512 0.006049] Line trace from player viewpoint and see if it intersects with a BPia
  ;;;[0.247 0.475 0.2664] Make sure isn't a hidden actor
  (bind _asbp_player_controller_2 (cast `/Game/Neurorama/Core/Player/BP_PlayerController` (`GameplayStatics.GetPlayerController` 0)))
  (bind _outhit_2 (`KismetSystemLibrary.LineTraceSingle` _returnvalue_2 (+ _returnvalue_2 (* (`SceneComponent.GetForwardVector` _mocon_r_arrow) 1000000.0)) "TraceTypeQuery1" true))
  (bind (_bblockinghit _binitialoverlap _time _distance _location _impactpoint _normal _impactnormal _physmat _hitactor) (`GameplayStatics.BreakHitResult` _outhit_2))
  (bind _asbp_info_actor_master (cast `/Game/Neurorama/Core/BP_infoActor_Master` _hitactor)
    (:`then`
      ;;[0.07819 0.1845 0.2831] Tell Diorama that owns hit object that it is hovered over it if it is an infoActor
      (bind _asbp_diorama_master (cast `/Game/Neurorama/Core/bp_Diorama_Master` (`self.GetParentActor` _hitactor))) ; Cast to diorama which owns the infoActor, because dioramas contain a lot of the UX/UI code for infoActor display methods, just to keep things organized
      (`/Game/Neurorama/Core/bp_Diorama_Master.hoverOverInfoActor` _asbp_diorama_master _asbp_info_actor_master)
      ;;[0.1044 0.42 0.09316] Reset visibility test array
      (`KismetArrayLibrary.Array_Clear` (`self.infoActorsIgnored`)))
    (:`CastFailed`
      ;;[0 0.3864 0.8796] If player hovers over something not an infoActor (i.e., the background) , tell all dioramas to unhover all infoActors
      (bind _asbp_game_instance (cast `/Game/Neurorama/Core/BP_GameInstance` (`GameplayStatics.GetGameInstance`)))
      (for _array_element (`/Game/Neurorama/Core/BP_GameInstance.dioramasCollected` _asbp_game_instance)
        (bind _asbp_diorama_master_2 (cast `/Game/Neurorama/Core/bp_Diorama_Master` _array_element))
        (`/Game/Neurorama/Core/bp_Diorama_Master.unhoverAllInfoActors` _asbp_diorama_master_2)))))

(fn `UserConstructionScript`)