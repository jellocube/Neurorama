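; VR test fly pawn for browsing dioramas, moved along camera-relative axes.
; Each tick it updates a laser beam and reports infoActors hit by the right controller's trace to their diorama for hover highlighting.
; Right trigger toggles selection and shows name and description, or deselects all dioramas on a miss.
; V respawns and possesses a BP_VR_Flypawn; thrust movement, yaw and unhover logic are disconnected.
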(event `InputAction|Action`
  (params (Key :type "Key Structure"))
  (bind _movementenabled (`self.movementEnabled`))
  ;[1 1 1] Mouse & Touchpad Movement Control
  (:`Pressed`
    (if _movementenabled :!label _label
      (set `self.Thrusting` true)))
  (:`Released`
    (if _movementenabled :!label _label_2
      (set `self.Thrusting` false))))

(event `InputTouch`
  (params (Location :type "Vector Structure") (FingerIndex :type "ETouchIndex Enum"))
  ;[1 1 1] Mouse & Touchpad Movement Control
  (:`Pressed`
    (goto _label))
  (:`Released`
    (goto _label_2)))

(event `InputAxis|LookUp`
  (params (AxisValue :type "Float (single-precision)"))
  ;[1 1 1] Look Control
  (`self.AddControllerPitchInput` AxisValue))

(event `InputAxis|MoveForward`
  (params (AxisValue :type "Float (single-precision)"))
  ;[1 1 1] Movement input basic
  (`self.AddMovementInput` (`KismetMathLibrary.GetForwardVector` (`KismetMathLibrary.MakeRotator` 0.0 (.pitch (`SceneComponent.RelativeRotation` (`self.Camera`))) (.yaw (`SceneComponent.RelativeRotation` (`self.Camera`))))) (* AxisValue -5.0)))

(event `InputAxis|Turn`
  (params (AxisValue :type "Float (single-precision)"))
  ;[1 1 1] Look Control
)

(event `InputAxis|MoveRight`
  (params (AxisValue :type "Float (single-precision)"))
  ;[1 1 1] Movement input basic
  (`self.AddMovementInput` (`KismetMathLibrary.GetRightVector` (`KismetMathLibrary.MakeRotator` 0.0 (.pitch (`SceneComponent.RelativeRotation` (`self.Camera`))) (.yaw (`SceneComponent.RelativeRotation` (`self.Camera`))))) (* AxisValue 5.0)))

(event `Key|MotionController_Right_Trigger`
  (params (Key :type "Key Structure"))
  (bind _mocon_r_arrow (`self.MoCon_R_Arrow`))
  (bind _returnvalue (`SceneComponent.K2_GetComponentLocation` _mocon_r_arrow))
  ;[1 1 1] Selection code
  ;;[0.1746 0.006512 0.006512] Click-to-select infoActor code
  (:`Released`
    (`self.isPawnControlled?`)
    (bind _outhit (`KismetSystemLibrary.LineTraceSingle` _returnvalue (+ _returnvalue (* (`SceneComponent.GetForwardVector` _mocon_r_arrow) 1000000.0)) "TraceTypeQuery2" false (`self.GetOverlappingActors` self null)))
    (bind (_bblockinghit _binitialoverlap _time _distance _location _impactpoint _normal _impactnormal _physmat _hitactor) (`GameplayStatics.BreakHitResult` _outhit))
    (bind _asbp_info_actor_master (cast `/Game/Neurorama/Core/BP_infoActor_Master` _hitactor)
      (:`then`
        ;;[0.0648 0.1651 0.2623] Tell Diorama that owns hit object to select it if it is an infoActor
        (bind _asbp_diorama_master (cast `/Game/Neurorama/Core/bp_Diorama_Master` (`self.GetParentActor` _asbp_info_actor_master)))
        (bind (_unselection_toggled _name _description _specialdescription _isdeselectingall) (`/Game/Neurorama/Core/bp_Diorama_Master.ToggleInfoActorSelection` _asbp_diorama_master _location _asbp_info_actor_master))
        (if (== _isdeselectingall true)
          ;;[0.7379 0.1912 0.3712] Update HUD Information
          (`SceneComponent.SetVisibility` (`self.textTitle`) false false :!label _label_3)
          (`SceneComponent.SetVisibility` (`self.textSubtitle`) false false)
          (else
            (bind _asbp_info_actor_master_2 (cast `/Game/Neurorama/Core/BP_infoActor_Master` _asbp_info_actor_master))
            (`TextRenderComponent.K2_SetText` (`self.textTitle`) (`/Game/Neurorama/Core/BP_infoActor_Master.Name` _asbp_info_actor_master_2))
            (`SceneComponent.SetVisibility` (`self.textTitle`) true false)
            (`TextRenderComponent.K2_SetText` (`self.textSubtitle`) (`/Game/Neurorama/Core/BP_infoActor_Master.Description` _asbp_info_actor_master_2))
            (`SceneComponent.SetVisibility` (`self.textSubtitle`) true false))))
      (:`CastFailed`
        ;;[0 0.3864 0.8796] If player clicks on something not an infoActor (i.e., the background) , tell all dioramas to deselct all infoActors
        (bind _asbp_game_instance (cast `/Game/Neurorama/Core/BP_GameInstance` (`GameplayStatics.GetGameInstance`)))
        (for _array_element (`/Game/Neurorama/Core/BP_GameInstance.dioramasCollected` _asbp_game_instance)
          (bind _asbp_diorama_master_2 (cast `/Game/Neurorama/Core/bp_Diorama_Master` _array_element))
          (`/Game/Neurorama/Core/bp_Diorama_Master.deselectAllInfoActors` _asbp_diorama_master_2)
          (goto _label_3))))))

(event `self.ReceiveTick`
  (params (DeltaSeconds :type "Float (single-precision)"))
  (bind _mocon_r_arrow (`self.MoCon_R_Arrow`))
  (bind _lasersource (`self.LaserSource`))
  (bind _laserbeam (`self.LaserBeam`))
  (bind _laserimpact (`self.LaserImpact`))
  (bind _returnvalue (`SceneComponent.K2_GetComponentLocation` _lasersource))
  (bind _returnvalue_2 (`SceneComponent.K2_GetComponentLocation` _mocon_r_arrow))
  (bind _returnvalue_3 (+ _returnvalue (* (`SceneComponent.GetForwardVector` _lasersource) 5000.0)))
  ;[1 1 1] Laser pointer code, based on https://www.youtube.com/watch?v=7VaMrs8n8e4&t=12s if i can bypass this when HMD is off, this pawn can be used for all sortsa stuff
  (`self.isPawnControlled?`)
  (bind (_outhit _returnvalue_4) (`KismetSystemLibrary.LineTraceSingle` _returnvalue _returnvalue_3 "TraceTypeQuery1"))
  (if _returnvalue_4
    (set `self.LaserTargetLoc` (`.Location` (`GameplayStatics.BreakHitResult` _outhit)))
    (else
      (bind _output_get (set `self.LaserTargetLoc` _returnvalue_3))))
  (`ParticleSystemComponent.SetBeamSourcePoint` _laserbeam 0 _returnvalue 0)
  (`ParticleSystemComponent.SetBeamTargetPoint` _laserbeam 0 _output_get 0)
  (`SceneComponent.K2_SetWorldLocation` _laserimpact (- _output_get (`SceneComponent.GetForwardVector` _laserimpact)) false false)
  ;[1 1 1] Lasterpointer-based hover-highlighting code
  ;;[0.1441 0.006512 0.006049] Line trace from player viewpoint and see if it intersects with a BPia
  (bind _outhit_2 (`KismetSystemLibrary.LineTraceSingle` _returnvalue_2 (+ _returnvalue_2 (* (`SceneComponent.GetForwardVector` _mocon_r_arrow) 1000000.0)) "TraceTypeQuery2" false (`self.GetOverlappingActors` self null)))
  (bind (_bblockinghit _binitialoverlap _time _distance _location _impactpoint _normal _impactnormal _physmat _hitactor) (`GameplayStatics.BreakHitResult` _outhit_2))
  (bind _asbp_info_actor_master (cast `/Game/Neurorama/Core/BP_infoActor_Master` _hitactor))
  ;;[0.07819 0.1845 0.2831] Tell Diorama that owns hit object that it is hovered over it if it is an infoActor
  (bind _asbp_diorama_master (cast `/Game/Neurorama/Core/bp_Diorama_Master` (`self.GetParentActor` _hitactor))) ; Cast to diorama which owns the infoActor, because dioramas contain a lot of the UX/UI code for infoActor display methods, just to keep things organized
  (`/Game/Neurorama/Core/bp_Diorama_Master.hoverOverInfoActor` _asbp_diorama_master _asbp_info_actor_master))

(event `Key|MotionController_Right_Trigger`
  (params (Key :type "Key Structure"))
  ;[1 1 1] Lasterpointer-based hover-highlighting code
  (:`Released`
    ;;[0.1441 0.006512 0.006049] Line trace from player viewpoint and see if it intersects with a BPia
    (`self.isPawnControlled?`)))

(event `Key|V`
  (params (Key :type "Key Structure"))
  (bind _returnvalue (`GameplayStatics.GetPlayerController` 0))
  ;[0.117 0.2346 0.1046] VR mode toggle
  (:`Released`
    (`Controller.UnPossess` _returnvalue)
    (`self.K2_DestroyActor`)
    (bind _returnvalue_2 (`|SpawnActorFromClass` "/Game/Neurorama/Core/Player/TestingVR/BP_VR_Flypawn.BP_VR_Flypawn_C" (`self.GetTransform` _returnvalue) "Undefined" "OverrideRootScale" null null))
    (`self.K2_TeleportTo` _returnvalue_2 (`self.K2_GetActorLocation`) (`self.K2_GetActorRotation`))
    (`Controller.Possess` (`GameplayStatics.GetPlayerController` 0) _returnvalue_2)))

(fn `UserConstructionScript`)